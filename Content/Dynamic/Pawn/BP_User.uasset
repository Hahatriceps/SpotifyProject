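; BP_User is a user pawn that records a short audio clip shortly after BeginPlay and hands it to the game instance as a prompt message.
; AudioCapture feeds a timed submix recording, which is exported as a WAV file to the project's Saved directory.
; After an on-screen file-exists check, the WAV is converted to a Google Speech JSON payload and passed to RegisterUserPromptMessage.
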(event `self.ReceiveBeginPlay`
  (`KismetSystemLibrary.Delay` 2.0)
  (`/Game/Dynamic/Interface/BPI_Recording.RecordAudio`))

(event `/Game/Dynamic/Interface/BPI_Recording.RecordAudio`
  (bind _returnvalue (`KismetStringLibrary.Concat_StrStr` (`KismetSystemLibrary.GetProjectSavedDirectory`) "Test2.wav"))
  (`KismetSystemLibrary.PrintString` "Start audio record ")
  (`SynthComponent.Start` (`self.AudioCapture`))
  (`AudioMixerBlueprintLibrary.StartRecordingOutput` 0.0 "/Game/Dynamic/Recording/Submix_Test.Submix_Test")
  (`KismetSystemLibrary.Delay` 5.0)
  (`SynthComponent.Stop` (`self.AudioCapture`))
  (`AudioMixerBlueprintLibrary.StopRecordingOutput` "WavFile" "Test2" (`KismetSystemLibrary.GetProjectSavedDirectory`) "/Game/Dynamic/Recording/Submix_Test.Submix_Test" null)
  (`KismetSystemLibrary.Delay` 0.5)
  (`KismetSystemLibrary.PrintString` (`KismetStringLibrary.Concat_StrStr` "File Exists: " (`KismetStringLibrary.Conv_BoolToString` (`BlueprintPathsLibrary.FileExists` _returnvalue))) true true (struct :`G` 0.66 :`B` 1.0 :`A` 1.0) 15.0)
  (bind _outjsonpayload (`BP_FileHelper.ConvertWavToJson` _returnvalue "GoogleSpeech" "Standard" false 48000 2))
  (message `/Game/Dynamic/Interface/BPI_Playback.RegisterUserPrompt` (`GameplayStatics.GetGameInstance`) _outjsonpayload))

(fn `UserConstructionScript`)